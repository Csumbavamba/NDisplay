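; BP_SwayCamera is a camera actor in LiveCapture that becomes player 0's view target and smoothly follows a tracked motion transform.
; BeginPlay finds BP_MotionTest and switches the view, or prints an error if none exists.
; Tick clears and re-finds that reference every frame, then uses TInterpTo to ease the actor toward its MotionRIght component's world transform at InterpolationSpeed.
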(event `self.ReceiveBeginPlay`
  (bind _returnvalue (`GameplayStatics.GetActorOfClass` "/Game/LiveCapture/BP_MotionTest.BP_MotionTest_C"))
  (bind _output_get (set `self.BP MotionTest` _returnvalue))
  (`/Engine/EditorBlueprintResources/StandardMacros.IsValid` _output_get
    (:`Is Valid`
      (`PlayerController.SetViewTargetWithBlend` (`GameplayStatics.GetPlayerController` 0) self 0.0 "VTBlend_Linear" 0.0 false))
    (:`Is Not Valid`
      (`KismetSystemLibrary.PrintString` "ERROR: Could not find motion Test BP" true true (struct :`R` 1.0 :`A` 1.0)))))

(event `self.ReceiveTick`
  (params (DeltaSeconds :type "Float (single-precision)"))
  (bind _output_get (set `self.BP MotionTest` null))
  (`/Engine/EditorBlueprintResources/StandardMacros.IsValid` _output_get
    (:`Is Valid`
      _)
    (:`Is Not Valid`
      (bind _returnvalue (`GameplayStatics.GetActorOfClass` "/Game/LiveCapture/BP_MotionTest.BP_MotionTest_C"))
      (set `self.BP MotionTest` _returnvalue)))
  (`self.K2_SetActorTransform` self (`KismetMathLibrary.TInterpTo` (`self.GetTransform`) (`SceneComponent.K2_GetComponentToWorld` (`/Game/LiveCapture/BP_MotionTest.MotionRIght` (`self.BP MotionTest`))) DeltaSeconds (`self.Interpolation Speed`)) false false))

(fn `UserConstructionScript`)